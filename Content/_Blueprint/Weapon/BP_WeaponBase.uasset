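; Base weapon Blueprint that provides shared fire and unequip behaviour for weapon actors.
; OnFireWeapon plays a gunshot sound and spawns a small explosion particle at the MuzzlePoint component, with no projectile or damage logic.
; OnUnequipped hides the skeletal mesh, destroys the actor and prints a debug message with its name.
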(event EventBeginPlay)

(event Collision|EventActorBeginOverlap
  (params (OtherActor :type Actor%20Object%20Reference)))

(event EventTick
  (params (DeltaSeconds :type Float%20%28single-precision%29)))

(event EventOnUnequipped
  (Rendering|SetVisibility (Variables|Default|GetSkeletalMesh) false false)
  (Actor|DestroyActor)
  (Development|PrintString (Utilities|String|Append (Utilities|GetObjectName self) " unequipped!")))

(event EventOnFireWeapon
  (bind _muzzlepoint (Variables|Default|GetMuzzlePoint))
  (bind _returnvalue (Transformation|GetWorldLocation _muzzlepoint))
  (Audio|PlaySoundatLocation "/Game/FirstPerson/Audio/FirstPersonTemplateWeaponFire02.FirstPersonTemplateWeaponFire02" _returnvalue "0, 0, 0" 0.5 1.0 0.0 0 0 0)
  (Effects|SpawnEmitteratLocation "/Game/StarterContent/Particles/P_Explosion.P_Explosion" _returnvalue "0, 0, 0" "0.100000,0.100000,0.100000"))

(fn ConstructionScript)